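; BP_HordeMode is a horde mode Blueprint that spawns AI trucks at locations chosen by the Environment Query System.
; SpawnAITruck runs the EQS_FindAISpawnLocation query from itself, picking randomly among the best 25 percent of results.
; On success, the query callback spawns BP_AITruck at the returned location with a fixed rotation, adjusting for collisions but always spawning.
; The construction script is empty, and NewFunction_0 only fetches query results without using them.
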(event `self.SpawnAITruck`
  (bind _returnvalue (`EnvQueryManager.RunEQSQuery` "/Game/AIQuery/EQS_FindAISpawnLocation.EQS_FindAISpawnLocation" self "RandomBest25Pct"))
  (add `EnvQueryInstanceBlueprintWrapper.OnQueryFinishedEvent` _returnvalue (delegate `OnQueryFinishedEvent_Event_0`)))

(event `OnQueryFinishedEvent_Event_0`
  (params (QueryInstance :type "EnvQueryInstanceBlueprintWrapper Object Reference") (QueryStatus :type "EEnvQueryStatus Enum" :default "Processing"))
  (switch `EEnvQueryStatus` QueryStatus
    (:`Success`
      ;[1 1 1] Query should return a single result on success, spawn actor at location.
      (bind _resultlocations (`EnvQueryInstanceBlueprintWrapper.GetQueryResultsAsLocations` QueryInstance))
      (`|SpawnActorFromClass` "/Game/Blueprints/Vehicles/BP_AITruck.BP_AITruck_C" (`KismetMathLibrary.MakeTransform` (`|GetArrayItem` _resultlocations) (struct :`Yaw` 90.0)) "AdjustIfPossibleButAlwaysSpawn" "OverrideRootScale" null null))))

(fn `NewFunction_0`
  (params (self2 :type "EnvQueryInstanceBlueprintWrapper Object Reference"))
  (`EnvQueryInstanceBlueprintWrapper.GetQueryResultsAsLocations` self2))

(fn `UserConstructionScript`)